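; BP_Dino is a player-controlled dino character that runs forward along world +X automatically and jumps on input.
; BeginPlay registers the IMC mapping context with the owning player controller's Enhanced Input subsystem.
; Tick applies constant movement input every frame, and the IA_Jump Started event triggers Jump.
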(event `self.ReceiveBeginPlay`
  (`self.AddInputMapping`))

(event `self.ReceiveTick`
  (params (DeltaSeconds :type "Float (single-precision)"))
  (`self.AddMovementInput` (1.0 0.0 0.0)))

(event `EnhancedInput|/Game/Input/IA_Jump`
  (params (ActionValue :type Boolean) (ElapsedSeconds :type "Float (double-precision)") (TriggeredSeconds :type "Float (double-precision)") (InputAction :type "InputAction Object Reference" :default "/Game/Input/IA_Jump.IA_Jump"))
  (:`Started`
    (`self.Jump`)))

(fn `AddInputMapping`
  (bind _asplayer_controller (cast `PlayerController` (`self.GetController`)))
  (bind _returnvalue (pcsubsystem `EnhancedInputLocalPlayerSubsystem` _asplayer_controller))
  (`/Engine/EditorBlueprintResources/StandardMacros.IsValid` _returnvalue
    (:`Is Valid`
      (`EnhancedInputSubsystemInterface.AddMappingContext` _returnvalue "/Game/Input/IMC.IMC" 0 (struct)))))

(fn `UserConstructionScript`)