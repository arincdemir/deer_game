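; Game mode for a dino endless runner that handles score, difficulty, spawning and the saved high score.
; Tick derives score from the dino's X distance, updates the UI and raises global time dilation along a sublinear real-time curve.
; ObstaclePassed spawns a random obstacle with a trigger ahead of the dino, while BackgroundPassed extends the scenery.
; ObstacleHit saves the high score, shows the end screen and pauses.
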(event `self.ReceiveBeginPlay`
  (bind _asbp_dino (cast `/Game/Blueprints/BP_Dino` (`GameplayStatics.GetPlayerPawn` 0)))
  (bind _output_get (set `self.BP Dino` _asbp_dino))
  (bind _returnvalue_x (`KismetMathLibrary.BreakVector` (`SceneComponent.K2_GetComponentLocation` (`Character.CapsuleComponent` _output_get))))
  (set `self.CharacterSpawnX` _returnvalue_x)
  (bind _returnvalue (`|CreateWidget` "/Game/Blueprints/WBP_GameUI.WBP_GameUI_C"))
  (bind _output_get_2 (set `self.UI` _returnvalue))
  (`UserWidget.AddToViewport` _output_get_2 0)
  (`self.SaveGameInit`))

(event `self.ReceiveTick`
  (params (DeltaSeconds :type "Float (single-precision)"))
  (bind _dilation (`self.TimeDilationRoot`))
  (`GameplayStatics.SetGlobalTimeDilation` _dilation)
  (`/Game/Blueprints/WBP_GameUI.UpdateUI` (`self.UI`) (`self.Score`) (`self.HighScore`))
  (bind _returnvalue (`self.CalculateScore`))
  (set `self.Score` _returnvalue))

(fn `Background Passed`
  (params (Background :type "/Game/Blueprints/BP_Background Object Reference"))
  (bind (_returnvalue_location _returnvalue_rotation _returnvalue_scale) (`KismetMathLibrary.BreakTransform` (`self.GetTransform` Background)))
  (set `self.LastBackground` Background)
  (`|SpawnActorFromClass` "/Game/Blueprints/BP_Background.BP_Background_C" (`KismetMathLibrary.MakeTransform` (+ _returnvalue_location (`KismetMathLibrary.MakeVector` (`self.BackgroundSpawnDistance`))) _returnvalue_rotation _returnvalue_scale) "Undefined" "MultiplyWithRoot" null null))

(fn `CalculateScore`
  (returns (ReturnValue :type Integer))
  (bind _returnvalue_x (`KismetMathLibrary.BreakVector` (`SceneComponent.K2_GetComponentLocation` (`Character.CapsuleComponent` (`self.BP Dino`)))))
  (return (`KismetMathLibrary.FTrunc` (/ (- _returnvalue_x (`self.CharacterSpawnX`)) 100.0))))

(fn `DeleteLastBackground`
  (`self.K2_DestroyActor` (`self.LastBackground`)))

(fn `ObstacleHit`
  (bind _savegame (`self.SaveGame`))
  (bind _savegameslot (`self.SaveGameSlot`))
  (set `/Game/Blueprints/BP_SaveGame.HighScore` (`KismetMathLibrary.Max` (`self.Score`) (`self.HighScore`)) _savegame)
  (`GameplayStatics.SaveGameToSlot` _savegame _savegameslot)
  (bind _returnvalue (`GameplayStatics.LoadGameFromSlot` _savegameslot))
  (cast `/Game/Blueprints/BP_SaveGame` _returnvalue)
  (`Widget.RemoveFromParent` (`self.UI`))
  (bind _returnvalue_2 (`|CreateWidget` "/Game/Blueprints/WBP_EndUI.WBP_EndUI_C"))
  (`/Game/Blueprints/WBP_EndUI.UpdateUI` _returnvalue_2 (`self.Score`) (`self.HighScore`))
  (`UserWidget.AddToViewport` _returnvalue_2 0)
  (`GameplayStatics.SetGamePaused` true)
  (set `PlayerController.bShowMouseCursor` true (`GameplayStatics.GetPlayerController` 0)))

(fn `ObstaclePassed`
  (bind _obstaclespawnxrandomness (`self.ObstacleSpawnXRandomness`))
  (bind _returnvalue_x (`KismetMathLibrary.BreakVector` (`SceneComponent.K2_GetComponentLocation` (`Character.CapsuleComponent` (`self.BP Dino`)))))
  (bind _output_get (set `self.ObstacleSpawnX` (+ (`KismetMathLibrary.RandomFloatInRange` _obstaclespawnxrandomness (* _obstaclespawnxrandomness -1.0)) (`self.ObstacleSpawnDistance`) _returnvalue_x)))
  (switch `int` (`KismetMathLibrary.RandomInteger` 3)
    (:`0`
      (bind _returnvalue (`KismetMathLibrary.MakeVector` _output_get 0.0 -60.0))
      (`self.SpawnOb1` _returnvalue))
    (:`1`
      (`self.SpawnOb2` _returnvalue))
    (:`2`
      (`self.SpawnOb3` _returnvalue)))
  (`|SpawnActorFromClass` "/Game/Blueprints/BP_Trigger.BP_Trigger_C" (`KismetMathLibrary.MakeTransform` (`KismetMathLibrary.MakeVector` (`self.ObstacleSpawnX`) 0.0 50.0)) "Undefined" "MultiplyWithRoot" null null))

(fn `SaveGameInit`
  (bind _returnvalue (`GameplayStatics.DoesSaveGameExist` (`self.SaveGameSlot`)))
  (if _returnvalue
    (bind _returnvalue_2 (`GameplayStatics.LoadGameFromSlot` (`self.SaveGameSlot`)))
    (bind _asbp_save_game (cast `/Game/Blueprints/BP_SaveGame` _returnvalue_2))
    (bind _output_get (set `self.SaveGame` _asbp_save_game))
    (set `self.HighScore` (`/Game/Blueprints/BP_SaveGame.HighScore` _output_get))
    (else
      (bind _returnvalue_3 (`GameplayStatics.CreateSaveGameObject` "/Game/Blueprints/BP_SaveGame.BP_SaveGame_C"))
      (bind _output_get_2 (set `self.SaveGame` _returnvalue_3))
      (`GameplayStatics.SaveGameToSlot` _output_get_2 (`self.SaveGameSlot`)))))

(fn `SpawnOb1`
  (params (Transform :type "Vector Structure"))
  (`|SpawnActorFromClass` "/Game/Blueprints/BP_Ob1.BP_Ob1_C" (`KismetMathLibrary.MakeTransform` Transform) "Undefined" "MultiplyWithRoot" null null))

(fn `SpawnOb2`
  (params (Transform :type "Vector Structure"))
  (`|SpawnActorFromClass` "/Game/Blueprints/BP_Ob2.BP_Ob2_C" (`KismetMathLibrary.MakeTransform` Transform) "Undefined" "MultiplyWithRoot" null null))

(fn `SpawnOb3`
  (params (Transform :type "Vector Structure"))
  (`|SpawnActorFromClass` "/Game/Blueprints/BP_Ob3.BP_Ob3_C" (`KismetMathLibrary.MakeTransform` Transform) "Undefined" "MultiplyWithRoot" null null))

(fn `TimeDilationLinear`
  (returns (Dilation :type "Float (double-precision)"))
  (return (+ (/ (`GameplayStatics.GetRealTimeSeconds`) 10.0) 1.0)))

(fn `TimeDilationRoot`
  (returns (Dilation :type "Float (double-precision)"))
  (return (+ (* (`KismetMathLibrary.MultiplyMultiply_FloatFloat` (`GameplayStatics.GetRealTimeSeconds`) 0.6) 0.125) 1.0)))

(fn `UserConstructionScript`)